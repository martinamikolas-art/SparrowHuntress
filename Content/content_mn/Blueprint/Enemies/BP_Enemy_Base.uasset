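; Base enemy character that provides sword combat animations, a patrol route getter and movement speed presets.
; Attack, wield and sheath events play montages, then fire event dispatchers when finished, with attack also reporting on interruption.
; Montage notifies time the spawning and hand-socket attachment of the sword actor, and its destruction on sheathing.
; SetMovementSpeed maps a speed state from idle to sprinting onto the character's max walk speed.
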(event `AttactPlayer`
  ;[1 1 1] AttackPlayer
  (`|PlayMontage` (`self.Mesh`) "/Game/content_mn/Animations/Slash_Sword.Slash_Sword"
    (:`OnCompleted`
      _)
    (:`OnInterrupted`
      _))
  (`self.OnAttackEnd`))

(event `WieldSword`
  ;[1 1 1] WieldSword
  (bind _notifyname (`|PlayMontage` (`self.Mesh`) "/Game/content_mn/Animations/Montage_Wield_Sword.Montage_Wield_Sword")
    (:`OnCompleted`
      (`self.OnWieldSword`))
    (:`OnNotifyBegin`
      (switch `name` _notifyname
        (:`WieldSword`
          (bind _returnvalue (`|SpawnActorFromClass` "/Game/content_mn/Blueprint/Weapons/BP_Sword.BP_Sword_C" (`self.GetTransform`) "Undefined" "MultiplyWithRoot" null null))
          (bind _output_get (set `self.SwordActor` _returnvalue))
          (`self.K2_AttachToComponent` _output_get (`self.Mesh`) "hand_r_sword_socket" "SnapToTarget" "SnapToTarget" "SnapToTarget" true)
          (set `self.IsWieldingSword` true))))))

(event `SheathSword`
  ;[1 1 1] SheathSword
  (bind _notifyname (`|PlayMontage` (`self.Mesh`) "/Game/content_mn/Animations/Montage_Sheath_Sword.Montage_Sheath_Sword")
    (:`OnCompleted`
      (`self.OnSheathSword`))
    (:`OnNotifyBegin`
      (switch `name` _notifyname
        (:`DropSword`
          (`self.K2_DestroyActor` (`self.SwordActor`))
          (set `self.IsWieldingSword` false))))))

(fn `GetPatrolRoute`
  (returns (PatrolRoute :type "/Game/content_mn/Blueprint/Enemies/AI/BP_PatrolRoute Object Reference"))
  (return (`self.PatrolRoute`)))

(fn `SetMovementSpeed`
  (params (Speed :type "/Game/content_mn/Blueprint/Enemies/AI/Enums/E_MovementSpeed Enum" :default "NewEnumerator0"))
  (returns (SpeedValue :type "Float (double-precision)"))
  (bind _output_get (set `CharacterMovementComponent.MaxWalkSpeed` (select `/Game/content_mn/Blueprint/Enemies/AI/Enums/E_MovementSpeed` Speed :`NewEnumerator1` 100.0 :`NewEnumerator2` 300.0 :`NewEnumerator3` 500.0 :!type "Float (single-precision)") (`self.CharacterMovement`)))
  (return _output_get))

(fn `UserConstructionScript`)